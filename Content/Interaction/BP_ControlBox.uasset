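; Interactable control box with clickable alarm, power and stop buttons, plus hinged USB and stop lids.
; Interacting toggles a replicated flag on the server, whose OnRep locks input, hides the player mesh, blends the view to the box and enables cursor clicks.
; Timelines animate the parts and drive lights and sound cues, with custom-depth highlights on hover.
; BackToGame blends the view back, then restores controls after a delay.
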(event `/Game/Interaction/BI_Interaction.InterfaceToggleFocus`
  (params (Focus :type Boolean))
  (`PrimitiveComponent.SetRenderCustomDepth` (`self.Control_Panel_Cube_001`) Focus))

(event `/Game/Interaction/BI_Interaction.InterfaceInteract`
  (`self.InteractOnServer`))

(event `InteractOnServer`
  (set `self.InteractToggle` (not (`self.InteractToggle`))))

(event `Delay`
  (params (Duration :type "Float (double-precision)"))
  (bind _returnvalue (`GameplayStatics.GetPlayerController` 0))
  (`KismetSystemLibrary.Delay` Duration)
  (`/Game/ThirdPerson/Blueprints/BP_ThirdPersonCharacter.SetMeshVisibility` (`self.Player`) true)
  (`Controller.SetIgnoreMoveInput` _returnvalue false)
  (`Controller.SetIgnoreLookInput` _returnvalue false)
  (`self.HideElements` false))

(event `self.btn_alarm.OnClicked`
  (params (TouchedComponent :type "PrimitiveComponent Object Reference") (ButtonPressed :type "Key Structure"))
  (bind _alarmlight (`self.AlarmLight`))
  ;[1 1 1] Alarm button logic
  (`ActorComponent.SetActive` (`self.open_Cue`) true false)
  (bind _output_get (set `self.isAlarmOn` (not (`self.isAlarmOn`))))
  (bind (_direction _newtrack_0) (`Timeline|alarm` :!via `PlayFromStart`)
    (:`Update`
      (`SceneComponent.K2_SetRelativeLocation` (`self.btn_alarm`) (`KismetMathLibrary.MakeVector` 0.0 _newtrack_0) false false)
      (`KismetSystemLibrary.Delay` 1.0)
      (`SceneComponent.SetVisibility` _alarmlight _output_get false)
      (if _output_get
        (bind (_direction_2 _newtrack_1) (`Timeline|lightFlicker` :!via `PlayFromStart` :!label _label)
          (:`Update`
            (`LightComponent.SetIntensity` _alarmlight _newtrack_1)
            (`ActorComponent.SetActive` (`self.alert_Cue`) _output_get false)))
        (else
          (goto _label :!via `Stop`))))))

(event `self.btn_alarm.OnBeginCursorOver`
  (params (TouchedComponent :type "PrimitiveComponent Object Reference"))
  ;[1 1 1] Alarm button logic
  (`PrimitiveComponent.SetRenderCustomDepth` (`self.btn_alarm`) true))

(event `self.btn_alarm.OnEndCursorOver`
  (params (TouchedComponent :type "PrimitiveComponent Object Reference"))
  ;[1 1 1] Alarm button logic
  (`PrimitiveComponent.SetRenderCustomDepth` (`self.btn_alarm`) false))

(event `self.btn_power.OnClicked`
  (params (TouchedComponent :type "PrimitiveComponent Object Reference") (ButtonPressed :type "Key Structure"))
  ;[1 1 1] Power button logic
  (`ActorComponent.SetActive` (`self.open_Cue`) true false)
  (bind _output_get (set `self.isPowerOn` (not (`self.isPowerOn`))))
  (bind (_direction _newtrack_0) (`Timeline|Timeline` :!via `PlayFromStart`)
    (:`Update`
      (`SceneComponent.K2_SetRelativeLocation` (`self.btn_power`) (`KismetMathLibrary.MakeVector` 0.0 _newtrack_0) false false)
      (`KismetSystemLibrary.Delay` 1.0)
      (`SceneComponent.SetVisibility` (`self.PowerLight`) _output_get false)
      (`ActorComponent.SetActive` (`self.pump_Cue`) _output_get false))))

(event `self.btn_power.OnBeginCursorOver`
  (params (TouchedComponent :type "PrimitiveComponent Object Reference"))
  ;[1 1 1] Power button logic
  (`PrimitiveComponent.SetRenderCustomDepth` (`self.btn_power`) true))

(event `self.btn_power.OnEndCursorOver`
  (params (TouchedComponent :type "PrimitiveComponent Object Reference"))
  ;[1 1 1] Power button logic
  (`PrimitiveComponent.SetRenderCustomDepth` (`self.btn_power`) false))

(event `self.USB_lid1.OnClicked`
  (params (TouchedComponent :type "PrimitiveComponent Object Reference") (ButtonPressed :type "Key Structure"))
  ;[1 1 1] USB1 lid logic
  (`ActorComponent.SetActive` (`self.open_Cue`) true false)
  (`/Engine/EditorBlueprintResources/StandardMacros.FlipFlop`
    (:`A`
      (bind (_direction _rotation _location_y _location_x) (`Timeline|Timeline_0` :!label _label_2)
        (:`Update`
          (`SceneComponent.K2_SetRelativeLocationAndRotation` (`self.USB_lid1`) (`KismetMathLibrary.MakeVector` _location_x _location_y 156.8) (`KismetMathLibrary.MakeRotator` 0.0 _rotation) false false))))
    (:`B`
      (goto _label_2 :!via `Reverse`))))

(event `self.USB_lid1.OnBeginCursorOver`
  (params (TouchedComponent :type "PrimitiveComponent Object Reference"))
  ;[1 1 1] USB1 lid logic
  (`PrimitiveComponent.SetRenderCustomDepth` (`self.USB_lid1`) true))

(event `self.USB_lid1.OnEndCursorOver`
  (params (TouchedComponent :type "PrimitiveComponent Object Reference"))
  ;[1 1 1] USB1 lid logic
  (`PrimitiveComponent.SetRenderCustomDepth` (`self.USB_lid1`) false))

(event `self.USB_lid2.OnClicked`
  (params (TouchedComponent :type "PrimitiveComponent Object Reference") (ButtonPressed :type "Key Structure"))
  ;[1 1 1] USB2 lid logic
  (`ActorComponent.SetActive` (`self.open_Cue`) true false)
  (`/Engine/EditorBlueprintResources/StandardMacros.FlipFlop`
    (:`A`
      (bind (_direction _rotation _location_y _location_x) (`Timeline|Timeline_1` :!label _label_3)
        (:`Update`
          (`SceneComponent.K2_SetRelativeLocationAndRotation` (`self.USB_lid2`) (`KismetMathLibrary.MakeVector` _location_x _location_y 144.0) (`KismetMathLibrary.MakeRotator` 0.0 _rotation) false false))))
    (:`B`
      (goto _label_3 :!via `Reverse`))))

(event `self.USB_lid2.OnBeginCursorOver`
  (params (TouchedComponent :type "PrimitiveComponent Object Reference"))
  ;[1 1 1] USB2 lid logic
  (`PrimitiveComponent.SetRenderCustomDepth` (`self.USB_lid2`) true))

(event `self.USB_lid2.OnEndCursorOver`
  (params (TouchedComponent :type "PrimitiveComponent Object Reference"))
  ;[1 1 1] USB2 lid logic
  (`PrimitiveComponent.SetRenderCustomDepth` (`self.USB_lid2`) false))

(event `self.Stop_lid.OnClicked`
  (params (TouchedComponent :type "PrimitiveComponent Object Reference") (ButtonPressed :type "Key Structure"))
  ;[1 1 1] Stop lid logic
  (`ActorComponent.SetActive` (`self.open_Cue`) true false)
  (`/Engine/EditorBlueprintResources/StandardMacros.FlipFlop`
    (:`A`
      (bind (_direction _rotation) (`Timeline|stopLid` :!label _label_4)
        (:`Update`
          (`SceneComponent.K2_SetRelativeRotation` (`self.Stop_lid`) (`KismetMathLibrary.MakeRotator` _rotation) false false))))
    (:`B`
      (goto _label_4 :!via `Reverse`))))

(event `self.btn_stop.OnClicked`
  (params (TouchedComponent :type "PrimitiveComponent Object Reference") (ButtonPressed :type "Key Structure"))
  ;[1 1 1] Stop button logic
  (`ActorComponent.SetActive` (`self.open_Cue`) true false)
  (bind (_direction _newtrack_0) (`Timeline|Timeline_2` :!via `PlayFromStart`)
    (:`Update`
      (`SceneComponent.K2_SetRelativeLocation` (`self.btn_stop`) (`KismetMathLibrary.MakeVector` 0.0 _newtrack_0) false false)
      (`KismetSystemLibrary.Delay` 1.0)
      (`SceneComponent.SetVisibility` (`self.PowerLight`) false false)
      (`ActorComponent.SetActive` (`self.pump_Cue`) false false)
      (set `self.isPowerOn` false))))

(event `self.btn_stop.OnBeginCursorOver`
  (params (TouchedComponent :type "PrimitiveComponent Object Reference"))
  ;[1 1 1] Stop button logic
  (`PrimitiveComponent.SetRenderCustomDepth` (`self.btn_stop`) true))

(event `self.btn_stop.OnEndCursorOver`
  (params (TouchedComponent :type "PrimitiveComponent Object Reference"))
  ;[1 1 1] Stop button logic
  (`PrimitiveComponent.SetRenderCustomDepth` (`self.btn_stop`) false))

(fn `backToGame`
  (if (`self.isInteracting`)
    (`PlayerController.SetViewTargetWithBlend` (`GameplayStatics.GetPlayerController` 0) (`self.Player`) 1.0 "VTBlend_Linear" 0.0 false)
    (`self.Delay` 0.8)
    (set `self.isInteracting` false)))

(fn `HideElements`
  (params (Hide :type Boolean))
  (bind _returnvalue (`GameplayStatics.GetPlayerController` 0))
  (bind _toexitpressbackspace (`/Game/ThirdPerson/Blueprints/BP_ThirdPersonCharacter.ToExitPressBackspace` (`self.Player`)))
  (bind _interactdot (`/Game/ThirdPerson/Blueprints/BP_ThirdPersonCharacter.InteractDot` (`self.Player`)))
  (set `PlayerController.bShowMouseCursor` Hide _returnvalue)
  (set `PlayerController.bEnableClickEvents` Hide _returnvalue)
  (set `PlayerController.bEnableMouseOverEvents` Hide _returnvalue)
  (`PrimitiveComponent.SetRenderCustomDepth` (`self.Control_Panel_Cube_001`) (not Hide))
  (`SceneComponent.SetHiddenInGame` (`self.Widget`) Hide false)
  (if Hide
    (`Widget.RemoveFromParent` _interactdot)
    (`UserWidget.AddToViewport` _toexitpressbackspace 0)
    (else
      (`UserWidget.AddToViewport` _interactdot 0)
      (`Widget.RemoveFromParent` _toexitpressbackspace))))

(fn `OnRep_InteractToggle`
  (bind _returnvalue (`GameplayStatics.GetPlayerController` 0))
  (bind _returnvalue_2 (`GameplayStatics.GetActorOfClass` "/Game/ThirdPerson/Blueprints/BP_ThirdPersonCharacter.BP_ThirdPersonCharacter_C"))
  (set `self.Player` _returnvalue_2)
  (if (`self.InteractToggle`)
    (`Controller.SetIgnoreLookInput` _returnvalue true)
    (`Controller.SetIgnoreMoveInput` _returnvalue true)
    (`/Game/ThirdPerson/Blueprints/BP_ThirdPersonCharacter.SetMeshVisibility` (`self.Player`) false)
    (`PlayerController.SetViewTargetWithBlend` _returnvalue self 1.0 "VTBlend_Linear" 0.0 false)
    (`self.HideElements` true)
    (set `self.isInteracting` true)
    (set `self.InteractToggle` false)))

(fn `UserConstructionScript`)