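; Interaction area variant whose shape is a custom static mesh.
; The construction script assigns the CustomShape mesh to the Shape component, then runs the parent construction script.
; When DEV is set, every material slot on the mesh gets the M_InteractionShapeTrace material; otherwise the shape is hidden without affecting its children.
; The event graph has no active logic.
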(fn `UserConstructionScript`
  (bind _shape (`self.Shape`))
  (`StaticMeshComponent.SetStaticMesh` (`self.Shape`) (`self.CustomShape`))
  (if (`self.DEV`)
    (for _array_element (`MeshComponent.GetMaterialSlotNames` _shape)
      (`PrimitiveComponent.SetMaterialByName` (`self.Shape`) _array_element "/Game/Interaction/InteractionArea/M_InteractionShapeTrace.M_InteractionShapeTrace"))
    (else
      (`SceneComponent.SetVisibility` _shape false false)))
  (`parent.UserConstructionScript`))